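; BP_Ball is a ball actor that moves along a Direction vector and bounces off whatever blocks it.
; Each Tick makes a swept offset, with speed capped at Speed and scaled by delta time.
; A blocking hit reflects Direction off the surface normal, sets CurrentSpeed from Speed times a decaying factor K, floored at MinSpeed, and prints it.
; The ReverseDirection, EditCurrentSpeed and EditK functions are unwired stubs.
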(event `self.ReceiveTick`
  (params (DeltaSeconds :type "Float (single-precision)"))
  (bind _sweephitresult (`self.K2_AddActorWorldOffset` (* (* (`self.Direction`) (`KismetMathLibrary.FMin` (`self.Current Speed`) (`self.Speed`))) DeltaSeconds) true))
  (bind (_bblockinghit _binitialoverlap _time _distance _location _impactpoint _normal) (`GameplayStatics.BreakHitResult` _sweephitresult))
  (if _bblockinghit
    ;[1 1 1] Set Vector Refflection
    (set `self.Direction` (`KismetMathLibrary.GetReflectionVector` (`self.Direction`) _normal))
    ;[1 1 1] Set Current Speed
    (bind _output_get (set `self.Current Speed` (`KismetMathLibrary.FMax` (* (`self.Speed`) (`self.K`)) (`self.Min Speed`))))
    (`KismetSystemLibrary.PrintString` (`KismetStringLibrary.Conv_DoubleToString` _output_get))
    ;[1 1 1] Set K
    (set `self.K` (- (`self.K`) 0.1))))

(fn `Edit Current Speed`)

(fn `Edit K`
  (returns (Output_Get :type "Float (double-precision)")))

(fn `Reverse Direction`
  (params (SurfaceNormal :type "Vector Structure")))

(fn `UserConstructionScript`)